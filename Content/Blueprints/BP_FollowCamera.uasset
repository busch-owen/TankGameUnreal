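; BP_FollowCamera is a shared camera actor that keeps two targets in frame.
; BeginPlay takes player 0's character as Target1, while Target2 is not assigned in these graphs.
; When both are valid, Tick moves the actor to their midpoint and sets the spring arm length to ArmLength plus half their separation.
; The construction script applies CameraAngle as the spring arm's relative rotation.
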(event EventTick
  (params (DeltaSeconds :type Float%20%28single-precision%29))
  (bind _target1 (Variables|Default|GetTarget1))
  (bind _target2 (Variables|Default|GetTarget2))
  (Utilities|IsValid _target1
    (:Is%20Valid
      (Utilities|IsValid _target2
        (:Is%20Valid
          (Transformation|SetActorLocation (/ (+ (Transformation|GetActorLocation _target1) (Transformation|GetActorLocation _target2)) 2.0) false false)
          (Variables|/Script/Engine.SpringArmComponent|SetTargetArmLength (Variables|Default|GetSpringArm) (CallFunction|SetFollowDistance)))))))

(event EventBeginPlay
  (Variables|Default|SetTarget1 (Game|GetPlayerCharacter 0)))

(fn ConstructionScript
  (Transformation|SetRelativeRotation (Variables|Default|GetSpringArm) (Variables|Default|GetCameraAngle) false false))

(fn SetFollowDistance
  (return (+ (Variables|Default|GetArmLength) (/ (Math|Vector|Distance(Vector) (Transformation|GetActorLocation (Variables|Default|GetTarget1)) (Transformation|GetActorLocation (Variables|Default|GetTarget2))) 2.0))))